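; A platformer spike floor obstacle that animates five spike rows one at a time in a repeating sequence while the level runs.
; LevelStart waits an initial delay, then a timeline lerps the current row's relative scale, with a sound played at the platform for each row.
; When the timeline finishes, it advances the index, wrapping after the last row, and replays.
; LevelEnd stops the timeline.
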(event EventLevelEnd
  ;[0.224 0.224 0.224] Spike Activation Timeline
  (bind _newtrack_0 (Timeline|Spike%20Speed Stop)
    (:Update
      (Transformation|SetRelativeScale3D (Utilities|Array|Get(acopy) (Variables|Default|GetSpikes) (Variables|Default|GetSpike%20Index)) (Math|Vector|Lerp(Vector) (Variables|Default|GetStart%20Scale) (Variables|Default|GetEnd%20Scale) _newtrack_0)))
    (:Finished
      (Math|Integer|IncrementInt (Variables|Default|GetSpike%20Index)
        (:%20%20
          (if (== 5 (Variables|Default|GetSpike%20Index))
            (Variables|Default|SetSpike%20Index 0))
          (Audio|PlaySoundatLocation "/Engine/VREditor/Sounds/UI/Object_Snaps_To_Grid.Object_Snaps_To_Grid" (Variables|Default|GetSound%20Location) "0, 0, 0" 0.7 1.0 0.0 "/Game/Platformer/Sounds/Attentuation/Spike_Attenuation.Spike_Attenuation" 0 0 0)
          (Timeline|Spike%20Speed PlayFromStart))))))

(event EventBeginPlay
  (Variables|Default|SetSound%20Location (Transformation|GetWorldLocation (Variables|Default|GetSM_Platform)))
  ;[0.224 0.224 0.224] Build Spike Array
  (Variables|Default|SetSpikes (Utilities|Array|MakeArray (Variables|Default|GetBP_SpikeRow1) (Variables|Default|GetBP_SpikeRow2) (Variables|Default|GetBP_SpikeRow3) (Variables|Default|GetBP_SpikeRow4) (Variables|Default|GetBP_SpikeRow5))))

(event EventLevelStart
  ;[0.224 0.224 0.224] Spike Activation Timeline
  (Utilities|FlowControl|Delay (Variables|Default|GetTimeline%20Delay))
  (if (== 5 (Variables|Default|GetSpike%20Index)) :!label _label
    (Variables|Default|SetSpike%20Index 0))
  (Audio|PlaySoundatLocation "/Engine/VREditor/Sounds/UI/Object_Snaps_To_Grid.Object_Snaps_To_Grid" (Variables|Default|GetSound%20Location) "0, 0, 0" 0.7 1.0 0.0 "/Game/Platformer/Sounds/Attentuation/Spike_Attenuation.Spike_Attenuation" 0 0 0)
  (bind _newtrack_0 (Timeline|Spike%20Speed PlayFromStart)
    (:Update
      (Transformation|SetRelativeScale3D (Utilities|Array|Get(acopy) (Variables|Default|GetSpikes) (Variables|Default|GetSpike%20Index)) (Math|Vector|Lerp(Vector) (Variables|Default|GetStart%20Scale) (Variables|Default|GetEnd%20Scale) _newtrack_0)))
    (:Finished
      (Math|Integer|IncrementInt (Variables|Default|GetSpike%20Index)
        (:%20%20
          (goto _label))))))

(fn ConstructionScript
  (|CallParentFunction))