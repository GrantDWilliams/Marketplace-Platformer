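; Platformer checkpoint that becomes the player's spawn point when BP_ThirdPersonCharacter overlaps its trigger.
; Swap deactivates the checkpoint stored in BP_GameInstance, registers itself and its SpawnPoint transform, turns its bulb green and plays a sound; deactivated bulbs turn red.
; On the first overlap only, it also sends LevelStartMessage to every BPI_LevelStage actor gathered at BeginPlay.
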(event OnComponentBeginOverlap(Trigger)
  (params (OverlappedComponent :type Primitive%20Component%20Object%20Reference) (OtherActor :type Actor%20Object%20Reference) (OtherComp :type Primitive%20Component%20Object%20Reference) (OtherBodyIndex :type Integer) (bFromSweep :type Boolean) (SweepResult :type Hit%20Result%20Structure%20%28by%20ref%29))
  ;[0.2865 0.2865 0.2865] Spawn Location Update
  (Utilities|Casting|CastToBP_ThirdPersonCharacter OtherActor)
  (CallFunction|Swap)
  ;[0.2292 0.2292 0.2292] Trigger Obstacles
  (Utilities|FlowControl|DoOnce false
    (:Completed
      (for _array_element (Variables|Default|GetTriggered%20Obstacles)
        (Class|BPILevelStage|LevelStart(Message) _array_element)))))

(event EventBeginPlay
  (CallFunction|BuildArray))

(fn ConstructionScript
  (Rendering|Material|SetVectorParameterValueonMaterials (Variables|Default|GetBulb) "Color" (Variables|Default|GetColor))
  (Rendering|Material|SetScalarParameterValueonMaterials (Variables|Default|GetBulb) "Glow Intensity" (Math|Conversions|ToFloat(Integer) (Variables|Default|GetGlowIntensity))))

(fn BuildArray
  (bind _outactors (Actor|GetAllActorswithInterface "/Game/Platformer/Interfaces/BPI_LevelStage.BPI_LevelStage_C"))
  (for _array_element _outactors
    (Utilities|Array|Add (Variables|Default|GetTriggered%20Obstacles) _array_element)))

(fn CheckActive
  (bind _bulb (Variables|Default|GetBulb))
  (if (Variables|Default|GetActive%20Checkpoint)
    (Rendering|Material|SetVectorParameterValueonMaterials _bulb "Color" "0.000000,1.000000,0.000000")
    (else
      (Rendering|Material|SetVectorParameterValueonMaterials _bulb "Color" "1.000000,0.000000,0.000000"))))

(fn Swap
  ;[0.3177 0.3177 0.3177] Validity Check
  (bind _asbp_game_instance (Utilities|Casting|CastToBP_GameInstance (Game|GetGameInstance)))
  (Utilities|IsValid (Variables|/Game/Platformer/BP_GameInstance.BP_GameInstance_C|GetCurrent%20Checkpoint _asbp_game_instance)
    (:Is%20Valid
      (if (not (== self (Variables|/Game/Platformer/BP_GameInstance.BP_GameInstance_C|GetCurrent%20Checkpoint _asbp_game_instance)))
        ;[0.3177 0.3177 0.3177] Set New Checkpoint
        (Variables|BP_Checkpoint_C|SetActive%20Checkpoint (Variables|/Game/Platformer/BP_GameInstance.BP_GameInstance_C|GetCurrent%20Checkpoint _asbp_game_instance) false)
        (CallFunction|CheckActive (Variables|/Game/Platformer/BP_GameInstance.BP_GameInstance_C|GetCurrent%20Checkpoint _asbp_game_instance))
        (Variables|/Game/Platformer/BP_GameInstance.BP_GameInstance_C|SetCurrent%20Checkpoint _asbp_game_instance self :!label _label)
        (Variables|Default|SetActive%20Checkpoint true)
        (Variables|/Game/Platformer/BP_GameInstance.BP_GameInstance_C|SetSpawn%20Transform _asbp_game_instance (Transformation|GetWorldTransform (Variables|Default|GetSpawn%20Point)))
        (CallFunction|CheckActive)
        (Audio|PlaySoundatLocation "/Engine/VREditor/Sounds/UI/Camera_Shutter.Camera_Shutter" "0, 0, 0" "0, 0, 0" 1.0 1.0 0.0 0 0 0 0)))
    (:Is%20Not%20Valid
      (goto _label))))