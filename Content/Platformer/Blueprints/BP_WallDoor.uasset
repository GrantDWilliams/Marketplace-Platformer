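; Sliding wall door for a platformer that opens once when its IntOpen event fires.
; A first timeline nudges it back along world X, then after a delay wired from that timeline's Update, a second slides it sideways along world Y, with a flag reversing the direction.
; Both stages move the actor by lerping between start and end locations, which are recomputed before the slide.
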(event EventBeginPlay)

(event Collision|EventActorBeginOverlap
  (params (OtherActor :type Actor%20Object%20Reference)))

(event EventTick
  (params (DeltaSeconds :type Float%20%28single-precision%29)))

(event EventIntOpen
  ;[0.1771 0.1771 0.1771] Opening Animation
  (Utilities|FlowControl|DoOnce false
    (:Completed
      (CallFunction|SetLocations)
      (bind _newtrack_0 (Timeline|Timeline PlayFromStart)
        (:Update
          (bind _movement (CallFunction|VectorLerp _newtrack_0))
          (Transformation|SetActorLocation _movement false false)
          (Utilities|FlowControl|Delay 2.5)
          (Variables|Default|SetStart%20Location (Variables|Default|GetEnd%20Location))
          (bind _slide_direction (CallFunction|CheckSlideDirection))
          (Variables|Default|SetEnd%20Location _slide_direction)
          (bind _newtrack_0_2 (Timeline|Timeline_0 Play)
            (:Update
              (bind _movement_2 (CallFunction|VectorLerp _newtrack_0_2))
              (Transformation|SetActorLocation _movement_2 false false))))))))

(fn ConstructionScript)

(fn CheckSlideDirection
  (bind _start_location (Variables|Default|GetStart%20Location))
  (return (select (Variables|Default|GetReverse%20Sliding%20Dir) (+ _start_location "0.000000,-480.000000,0.000000") (+ _start_location "0.000000,480.000000,0.000000"))))

(fn SetLocations
  (Variables|Default|SetStart%20Location (Transformation|GetActorLocation))
  (Variables|Default|SetEnd%20Location (+ "-30.000000,0.000000,0.000000" (Variables|Default|GetStart%20Location))))

(fn VectorLerp
  (params (Alpha :type Float%20%28double-precision%29))
  (return (Math|Vector|Lerp(Vector) (Variables|Default|GetStart%20Location) (Variables|Default|GetEnd%20Location) Alpha)))