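; BP_GlowPlane is a platformer lighting actor built around a 2D plane mesh with a configurable glow.
; The construction script pushes the EmissiveIntensity and Color variables into the plane's GlowIntensity and Color material parameters.
; On BeginPlay it plays the Light02 sound quietly at the plane's world location.
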(event EventBeginPlay
  (Audio|PlaySoundatLocation "/Game/StarterContent/Audio/Light02.Light02" (Transformation|GetWorldLocation (Variables|Default|Get2dPlane)) "0, 0, 0" 0.1 1.0 0.0 0 0 0 0))

(fn ConstructionScript
  (Rendering|Material|SetScalarParameterValueonMaterials (Variables|Default|Get2dPlane) "GlowIntensity" (Math|Conversions|ToFloat(Integer) (Variables|Default|GetEmissiveIntensity)))
  (Rendering|Material|SetVectorParameterValueonMaterials (Variables|Default|Get2dPlane) "Color" (Variables|Default|GetColor)))