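; Kill obstacle base logic for the platformer that runs the player death sequence when KillPlayer is called.
; BeginPlay caches the first PostProcessVolume and, if no death camera is set, a Default-tagged CCTV.
; KillPlayer notifies BPI_LevelStage actors, stops music, switches to the death camera and flashes red through timeline-driven post-process gain.
; A DoOnce then plays an alarm, shows the death screen and reloads the level after delays.
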(event Custom|Kill%20Player
  (bind _post_process_ref (Variables|Default|GetPost%20Process%20Ref))
  (bind _outactors (Actor|GetAllActorswithInterface "/Game/Platformer/Interfaces/BPI_LevelStage.BPI_LevelStage_C"))
  (for _array_element _outactors
    (Class|BPILevelStage|LevelEnd(Message) _array_element)
    (bind _asbp_third_person_game_mode (Utilities|Casting|CastToBP_ThirdPersonGameMode (Game|GetGameMode)))
    (Audio|Components|Audio|Stop (Variables|/Game/ThirdPerson/Blueprints/BP_ThirdPersonGameMode.BP_ThirdPersonGameMode_C|GetBackground%20Music _asbp_third_person_game_mode))
    ;[0.2865 0.2865 0.2865] Death Camera
    (Game|Player|SetViewTargetwithBlend (Game|GetPlayerController (Game|GetPlayerState 0)) (Variables|Default|GetDeathCam%20Ref) 0.0 "VTBlend_Linear" 0.0 false)
    ;[0.2865 0.2865 0.2865] Red Flash
    (bind _red_flash (Timeline|Timeline_0 PlayFromStart)
      (:Update
        (bind _structout (Utilities|Struct|SetmembersinPostProcessSettings (Variables|/Script/Engine.PostProcessVolume|GetSettings _post_process_ref) (Math|Vector4|MakeVector4 2.0 0.7 0.7 _red_flash)))
        (Variables|/Script/Engine.PostProcessVolume|SetSettings _post_process_ref _structout)
        ;[0.2865 0.2865 0.2865] Death Screen, Sound, & Respawn
        (Utilities|FlowControl|DoOnce false
          (:Completed
            (Audio|PlaySound2D "/Game/Platformer/Sounds/alarm-62609.alarm-62609" 0.6 1.0 0.0 0 0)
            (Utilities|FlowControl|Delay 4.0)
            (bind _returnvalue (UserInterface|CreateWidget "/Game/Platformer/UI/WBP_DeathScreen.WBP_DeathScreen_C"))
            (UserInterface|Viewport|AddtoViewport _returnvalue 0)
            (Utilities|FlowControl|Delay 4.0)
            (Game|OpenLevel(byName) "Platformer")))))))

(event EventBeginPlay
  ;[0.2865 0.2865 0.2865] Sets default PostProcessVolume & DeathCam if not set manually.
  (bind _outactors (Actor|GetAllActorsOfClass "/Script/Engine.PostProcessVolume"))
  (Variables|Default|SetPost%20Process%20Ref (Utilities|Array|Get(acopy) _outactors))
  (if (not (Utilities|IsValid (Variables|Default|GetDeathCam%20Ref)))
    (bind _outactors_2 (Actor|GetAllActorsOfClasswithTag "/Game/Platformer/Blueprints/BP_CCtv.BP_CCtv_C" "Default"))
    (Variables|Default|SetDeathCam%20Ref (Utilities|Array|Get(acopy) _outactors_2))))

(fn ConstructionScript
  (|CallParentFunction))