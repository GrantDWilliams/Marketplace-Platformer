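; Platformer obstacle actor that moves or rotates between a start and end pose.
; LevelStart marks it active and caches its current location and rotation as the start pose.
; ApplyTimeAlpha takes an externally supplied alpha and, based on UseRotator, lerps either rotation toward an absolute end rotation or location toward an offset relative to the start, without sweeping.
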(event EventLevelStart
  (Variables|Default|SetIs%20Active true)
  (Variables|Default|SetStart%20Vector (Transformation|GetActorLocation))
  (Variables|Default|SetStart%20Rotation (Transformation|GetActorRotation)))

(fn ConstructionScript)

(fn ApplyTimeAlpha
  (params (Alpha :type Float%20%28double-precision%29))
  (bind _start_vector (Variables|Default|GetStart%20Vector))
  (if (Variables|Default|GetUse%20Rotator)
    (Transformation|SetActorRotation (Math|Rotator|Lerp(Rotator) (Variables|Default|GetStart%20Rotation) (Variables|Default|GetEnd%20Rotation) Alpha))
    (else
      (Transformation|SetActorLocation (Math|Vector|Lerp(Vector) _start_vector (+ _start_vector (Variables|Default|GetEnd%20Vector)) Alpha) false false))))