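; BP_Killbox is a platformer kill volume that triggers the death sequence when BP_ThirdPersonCharacter overlaps it.
; It disables the character's input and blends the view to a death camera.
; A timeline drives a red-tinted color gain on the referenced post process settings, while a DoOnce fires the alarm sound.
; After a delay it shows WBP_DeathScreen, then after another reloads the Platformer level.
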(event OnComponentBeginOverlap(Killbox)
  (params (OverlappedComponent :type Primitive%20Component%20Object%20Reference) (OtherActor :type Actor%20Object%20Reference) (OtherComp :type Primitive%20Component%20Object%20Reference) (OtherBodyIndex :type Integer) (bFromSweep :type Boolean) (SweepResult :type Hit%20Result%20Structure%20%28by%20ref%29))
  (bind _post_process_ref (Variables|Default|GetPost%20Process%20Ref))
  (bind _asbp_third_person_character (Utilities|Casting|CastToBP_ThirdPersonCharacter OtherActor))
  (Input|DisableInput _asbp_third_person_character 0)
  ;[0.2292 0.2292 0.2292] Death Camera
  (Game|Player|SetViewTargetwithBlend (Game|GetPlayerController (Game|GetPlayerState 0)) (Variables|Default|GetDeathCam%20Ref) 0.0 "VTBlend_Linear" 0.0 false)
  ;[0.2865 0.2865 0.2865] Red Flash
  (bind _red_flash (Timeline|Timeline PlayFromStart)
    (:Update
      (bind _structout (Utilities|Struct|SetmembersinPostProcessSettings (Variables|/Script/Engine.PostProcessVolume|GetSettings _post_process_ref) (Math|Vector4|MakeVector4 2.0 0.7 0.7 _red_flash)))
      (Variables|/Script/Engine.PostProcessVolume|SetSettings _post_process_ref _structout)
      (Utilities|FlowControl|DoOnce false
        (:Completed
          (Audio|PlaySound2D "/Game/Platformer/Sounds/alarm-62609.alarm-62609" 0.6 1.0 0.0 0 0)
          (Utilities|FlowControl|Delay 8.0)
          (bind _returnvalue (UserInterface|CreateWidget "/Game/Platformer/UI/WBP_DeathScreen.WBP_DeathScreen_C"))
          (UserInterface|Viewport|AddtoViewport _returnvalue 0)
          (Utilities|FlowControl|Delay 8.0)
          (Game|OpenLevel(byName) "Platformer"))))))

(fn ConstructionScript)