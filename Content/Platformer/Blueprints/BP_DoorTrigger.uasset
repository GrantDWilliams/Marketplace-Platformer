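; BP_DoorTrigger is a one-shot trigger volume that tells doors to open when anything begins overlapping its box.
; It finds every actor implementing BPI_DoorTrigger and sends the open message through that interface, with no direct door references.
; It then plays three timed sound effects, separated by delays, at the root's world location plus the SoundWidget offset.
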(event OnComponentBeginOverlap(Box)
  (params (OverlappedComponent :type Primitive%20Component%20Object%20Reference) (OtherActor :type Actor%20Object%20Reference) (OtherComp :type Primitive%20Component%20Object%20Reference) (OtherBodyIndex :type Integer) (bFromSweep :type Boolean) (SweepResult :type Hit%20Result%20Structure%20%28by%20ref%29))
  ;[0.2344 0.2344 0.2344] Doors told to open.
  (Utilities|FlowControl|DoOnce false
    (:Completed
      (bind _outactors (Actor|GetAllActorswithInterface "/Game/Platformer/Interfaces/BPI_DoorTrigger.BPI_DoorTrigger_C"))
      (Class|BPIDoorTrigger|IntOpen(Message) _outactors)
      ;[0.2344 0.2344 0.2344] Sounds effects played at collision location.
      (bind _sound_world_location (CallFunction|SoundWorldLocation))
      (Audio|PlaySoundatLocation "/Engine/EditorSounds/GamePreview/StartSimulate.StartSimulate" _sound_world_location "0, 0, 0" 0.5 1.0 0.0 0 0 0 0)
      (Utilities|FlowControl|Delay 2.5)
      (Audio|PlaySoundatLocation "/Engine/VREditor/Sounds/UI/Dockable_Window_Open.Dockable_Window_Open" _sound_world_location "0, 0, 0" 1.0 1.0 0.0 0 0 0 0)
      (Utilities|FlowControl|Delay 3.0)
      (Audio|PlaySoundatLocation "/Engine/EditorSounds/GamePreview/EndPlayInEditor.EndPlayInEditor" _sound_world_location "0, 0, 0" 0.5 1.0 0.0 0 0 0 0))))

(fn ConstructionScript)

(fn SoundWorldLocation
  (return (+ (Transformation|GetWorldLocation (Variables|Default|GetDefaultSceneRoot)) (Variables|Default|GetSound%20Widget))))