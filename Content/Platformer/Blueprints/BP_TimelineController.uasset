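; BP_TimelineController drives every Obstacle in a level from one shared, ping-ponging timeline.
; It gathers the Obstacle actors at BeginPlay and starts cycling on LevelStart, passing the timeline alpha to each obstacle's ApplyTimeAlpha on every update.
; A FlipFlop alternates forward and reverse playback, looping through the Finished pin after a configurable delay, with play rate derived from TimelineLength.
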(event EventLevelStart
  (Utilities|FlowControl|Delay (Variables|Default|GetTimeline%20Delay) :!label _label)
  (Components|Timeline|SetPlayRate (Variables|Default|GetTimeline) (/ 1.0 (Variables|Default|GetTimeline%20Length)))
  (Utilities|FlowControl|FlipFlop
    (:A
      (bind _alpha (Timeline|Timeline PlayFromStart)
        (:Update
          (for _array_element (Variables|Default|GetObstacles)
            (bind _asobstacle (Utilities|Casting|CastToObstacle _array_element))
            (Default|ApplyTimeAlpha _asobstacle _alpha)))
        (:Finished
          (goto _label))))
    (:B
      (Timeline|Timeline ReverseFromEnd))))

(event EventBeginPlay
  (bind _outactors (Actor|GetAllActorsOfClass "/Game/Platformer/Blueprints/Classes/Obstacle.Obstacle_C"))
  (Variables|Default|SetObstacles _outactors))

(fn ConstructionScript)